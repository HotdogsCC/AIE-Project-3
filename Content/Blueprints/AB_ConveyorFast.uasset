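; AB_ConveyorFast is a conveyor actor that carries whatever overlaps its Box along the direction of its Arrow component.
; Each Tick it offsets every overlapping actor by the Arrow's forward vector, scaled by Speed and DeltaSeconds, without sweeping.
; On BeginPlay it waits 25 seconds, then teleports itself to a hardcoded world location; the GetAllActorsOfClass result there is unused.
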(event EventBeginPlay
  (Utilities|FlowControl|Delay 25.0)
  (Actor|GetAllActorsOfClass "AB_ConveyorFast_C")
  (Transformation|SetActorLocation "1490.000000,1660.000000,520.000000" false true))

(event EventTick
  (params (DeltaSeconds :type Float%20%28single-precision%29))
  ;[1 0.7365 0.115] Conveyor Overlapping Actor Targetted Movement
  (for _array_element (Collision|GetOverlappingActors (Variables|Default|GetBox) 0 :!class /Script/Engine.PrimitiveComponent)
    (Transformation|AddActorWorldOffset _array_element (* (Math|Vector|GetForwardVector (Transformation|GetWorldRotation (Variables|Default|GetArrow))) (* DeltaSeconds (Variables|Default|GetSpeed))))))

(fn ConstructionScript)