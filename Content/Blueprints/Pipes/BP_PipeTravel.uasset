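; BP_PipeTravel is a trigger actor for pipe travel that takes over a character on overlap and launches it out at the end.
; On overlap it zeroes the character's velocity and gravity, disables input, then calls StartTravelling, whose movement logic is not in this graph.
; The Eject event restores a fixed gravity scale, applies a heavily scaled directional force through CharacterMovement and re-enables input.
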(event EventEject
  (params (InCharacter :type Actor%20Object%20Reference) (ForceDirection :type Vector :default "0, 0, 0") (Force :type Float%20%28single-precision%29))
  (bind _ascharacter (Utilities|Casting|CastToCharacter InCharacter)) ; make the object a character
  (Variables|/Script/Engine.CharacterMovementComponent|SetGravityScale (Variables|/Script/Engine.Character|GetCharacterMovement _ascharacter) 1.75)
  (Physics|AddForce (Variables|/Script/Engine.Character|GetCharacterMovement _ascharacter) (* (* ForceDirection Force) 1e+07))
  (Input|EnableInput _ascharacter 0))

(event Collision|EventActorBeginOverlap
  (params (OtherActor :type Actor%20Object%20Reference))
  (bind _ascharacter (Utilities|Casting|CastToCharacter OtherActor)) ; check the object is a character
  (Variables|/Script/Engine.MovementComponent|SetVelocity (Variables|/Script/Engine.Character|GetCharacterMovement _ascharacter) "0, 0, 0") ; resets player velocity
  (Variables|/Script/Engine.CharacterMovementComponent|SetGravityScale (Variables|/Script/Engine.Character|GetCharacterMovement _ascharacter) 0.0) ; make player temp not have gravity
  (Input|DisableInput _ascharacter 0) ; stop the player from controlling the character
  (Class|PipeTravel|StartTravelling OtherActor))

(fn ConstructionScript)