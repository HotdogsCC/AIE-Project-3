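; BP_Bomb is a timed bomb actor that plays a ticking sound from BeginPlay and explodes after a fixed fuse delay.
; A Timeline's Update output activates the Niagara effect and explosion sound, then after a short delay enlarges the Sphere and immediately destroys the actor.
; The Sphere transform node and scale interpolation are disconnected, so the Timeline animates nothing.
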(event EventBeginPlay
  (Audio|PlaySound2D "/Game/Sounds/BombTicking.BombTicking" 1.0 1.0 0.0 0 0)
  (Utilities|FlowControl|Delay 3.4)
  (bind _alpha (Timeline|Timeline Play)
    (:Update
      (Components|Activation|Activate (Variables|Default|GetNiagara) false)
      (Audio|PlaySound2D "/Game/Sounds/BombExplosion2.BombExplosion2" 1.0 1.0 0.0 0 0)
      (Utilities|FlowControl|Delay 0.4)
      (Transformation|SetWorldScale3D (Variables|Default|GetSphere) "10.000000,10.000000,10.000000")
      (Actor|DestroyActor))))

(fn ConstructionScript)