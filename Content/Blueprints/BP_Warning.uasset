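; Warning light actor that sounds an alarm and flashes at two scripted moments after play begins.
; BeginPlay runs one linear chain of Delays, firing first a few seconds in and again roughly fifteen seconds after the first burst.
; Each burst plays a 2D alarm and blinks the Sphere and Cylinder meshes by swapping their material between MI_FlashingLight and MI_Factory.
; The timing is hardcoded with no loop, timer or external trigger.
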(event EventBeginPlay
  (Utilities|FlowControl|Delay 6.0)
  (Audio|PlaySound2D "/Game/Sounds/Alarm.Alarm" 1.0 1.0 0.0 0 0)
  (Rendering|Material|SetMaterial (Variables|Default|GetSphere) 0 "/Game/Materials/MI_FlashingLight.MI_FlashingLight")
  (Rendering|Material|SetMaterial (Variables|Default|GetCylinder) 0 "/Game/Materials/MI_FlashingLight.MI_FlashingLight")
  (Utilities|FlowControl|Delay 0.25)
  (Rendering|Material|SetMaterial (Variables|Default|GetSphere) 0 "/Game/Materials/MI_Factory.MI_Factory")
  (Rendering|Material|SetMaterial (Variables|Default|GetCylinder) 0 "/Game/Materials/MI_Factory.MI_Factory")
  (Utilities|FlowControl|Delay 0.25)
  (Rendering|Material|SetMaterial (Variables|Default|GetSphere) 0 "/Game/Materials/MI_FlashingLight.MI_FlashingLight")
  (Rendering|Material|SetMaterial (Variables|Default|GetCylinder) 0 "/Game/Materials/MI_FlashingLight.MI_FlashingLight")
  (Utilities|FlowControl|Delay 0.25)
  (Rendering|Material|SetMaterial (Variables|Default|GetSphere) 0 "/Game/Materials/MI_Factory.MI_Factory")
  (Rendering|Material|SetMaterial (Variables|Default|GetCylinder) 0 "/Game/Materials/MI_Factory.MI_Factory")
  (Utilities|FlowControl|Delay 0.25)
  (Rendering|Material|SetMaterial (Variables|Default|GetSphere) 0 "/Game/Materials/MI_FlashingLight.MI_FlashingLight")
  (Rendering|Material|SetMaterial (Variables|Default|GetCylinder) 0 "/Game/Materials/MI_FlashingLight.MI_FlashingLight")
  (Utilities|FlowControl|Delay 0.25)
  (Rendering|Material|SetMaterial (Variables|Default|GetSphere) 0 "/Game/Materials/MI_Factory.MI_Factory")
  (Rendering|Material|SetMaterial (Variables|Default|GetCylinder) 0 "/Game/Materials/MI_Factory.MI_Factory")
  (Utilities|FlowControl|Delay 0.25)
  (Rendering|Material|SetMaterial (Variables|Default|GetSphere) 0 "/Game/Materials/MI_FlashingLight.MI_FlashingLight")
  (Rendering|Material|SetMaterial (Variables|Default|GetCylinder) 0 "/Game/Materials/MI_FlashingLight.MI_FlashingLight")
  (Utilities|FlowControl|Delay 0.25)
  (Rendering|Material|SetMaterial (Variables|Default|GetSphere) 0 "/Game/Materials/MI_Factory.MI_Factory")
  (Rendering|Material|SetMaterial (Variables|Default|GetCylinder) 0 "/Game/Materials/MI_Factory.MI_Factory")
  (Utilities|FlowControl|Delay 15.2)
  (Audio|PlaySound2D "/Game/Sounds/Alarm.Alarm" 1.0 1.0 0.0 0 0)
  (Rendering|Material|SetMaterial (Variables|Default|GetSphere) 0 "/Game/Materials/MI_FlashingLight.MI_FlashingLight")
  (Rendering|Material|SetMaterial (Variables|Default|GetCylinder) 0 "/Game/Materials/MI_FlashingLight.MI_FlashingLight")
  (Utilities|FlowControl|Delay 0.25)
  (Rendering|Material|SetMaterial (Variables|Default|GetSphere) 0 "/Game/Materials/MI_Factory.MI_Factory")
  (Rendering|Material|SetMaterial (Variables|Default|GetCylinder) 0 "/Game/Materials/MI_Factory.MI_Factory")
  (Utilities|FlowControl|Delay 0.25)
  (Rendering|Material|SetMaterial (Variables|Default|GetSphere) 0 "/Game/Materials/MI_FlashingLight.MI_FlashingLight")
  (Rendering|Material|SetMaterial (Variables|Default|GetCylinder) 0 "/Game/Materials/MI_FlashingLight.MI_FlashingLight")
  (Utilities|FlowControl|Delay 0.25)
  (Rendering|Material|SetMaterial (Variables|Default|GetSphere) 0 "/Game/Materials/MI_Factory.MI_Factory")
  (Rendering|Material|SetMaterial (Variables|Default|GetCylinder) 0 "/Game/Materials/MI_Factory.MI_Factory")
  (Utilities|FlowControl|Delay 0.25)
  (Rendering|Material|SetMaterial (Variables|Default|GetSphere) 0 "/Game/Materials/MI_FlashingLight.MI_FlashingLight")
  (Rendering|Material|SetMaterial (Variables|Default|GetCylinder) 0 "/Game/Materials/MI_FlashingLight.MI_FlashingLight")
  (Utilities|FlowControl|Delay 0.25)
  (Rendering|Material|SetMaterial (Variables|Default|GetSphere) 0 "/Game/Materials/MI_Factory.MI_Factory")
  (Rendering|Material|SetMaterial (Variables|Default|GetCylinder) 0 "/Game/Materials/MI_Factory.MI_Factory")
  (Utilities|FlowControl|Delay 0.25)
  (Rendering|Material|SetMaterial (Variables|Default|GetSphere) 0 "/Game/Materials/MI_FlashingLight.MI_FlashingLight")
  (Rendering|Material|SetMaterial (Variables|Default|GetCylinder) 0 "/Game/Materials/MI_FlashingLight.MI_FlashingLight")
  (Utilities|FlowControl|Delay 0.25)
  (Rendering|Material|SetMaterial (Variables|Default|GetSphere) 0 "/Game/Materials/MI_Factory.MI_Factory")
  (Rendering|Material|SetMaterial (Variables|Default|GetCylinder) 0 "/Game/Materials/MI_Factory.MI_Factory"))

(fn ConstructionScript)