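; BP_SafeGuard is a spinning pickup for the Death Swap minigame that grants a safeguard to the player who touches it.
; It rotates continuously on yaw every tick.
; When a minigame character overlaps it, it registers that player with the BPMG_DeathSwap game mode, plays a 2D sound and destroys itself.
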(event EventTick
  (params (DeltaSeconds :type Float%20%28single-precision%29))
  (Transformation|AddActorLocalRotation (Math|Rotator|MakeRotator 0.0 0.0 (* DeltaSeconds (Math|Float|MakeLiteralFloat -9e+01))) false false))

(event Collision|EventActorBeginOverlap
  (params (OtherActor :type Actor%20Object%20Reference))
  (bind _asminigame_character_base (Utilities|Casting|CastToMinigameCharacterBase OtherActor))
  (bind _asbpmg_death_swap (Utilities|Casting|CastToBPMG_DeathSwap (Game|GetGameMode)))
  (Class|MinigameDeathSwap|SetPlayerwithSafeGuard _asbpmg_death_swap _asminigame_character_base)
  (Audio|PlaySound2D "/Game/Sounds/Cues/SafeGuard_Cue.SafeGuard_Cue" 1.0 1.0 0.0 0 0)
  (Actor|DestroyActor))

(fn ConstructionScript)